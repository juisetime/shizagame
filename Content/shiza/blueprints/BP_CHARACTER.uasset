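; First-person player character that adds its two UI widgets and Enhanced Input context on BeginPlay, then handles movement with camera shake, look and jump.
; Left click triggers the Bp_Fonariks (flashlight) actor; click and look are ignored while the cursor shows.
; A 500-unit camera trace flags hover over bp_gl interactables each Tick.
; E uses bp_gl_stable objects or picks up one other bp_gl at a time, which the drop input releases.
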(event `self.ReceiveBeginPlay`
  (bind _returnvalue (`|CreateWidget` "/Game/shiza/vidgets/HELPUSER_UI.HELPUSER_UI_C"))
  (bind _returnvalue_2 (`|CreateWidget` "/Game/shiza/vidgets/vidget_password.vidget_password_C"))
  (bind _output_get (set `self.NewVar` _returnvalue_2))
  (`UserWidget.AddToViewport` _returnvalue 0)
  (`UserWidget.AddToViewport` _output_get 0)
  (bind _asplayer_controller (cast `PlayerController` (`GameplayStatics.GetPlayerController` 0)))
  (bind _returnvalue_3 (pcsubsystem `EnhancedInputLocalPlayerSubsystem` _asplayer_controller))
  (`/Engine/EditorBlueprintResources/StandardMacros.IsValid` _returnvalue_3
    (:`Is Valid`
      (`EnhancedInputSubsystemInterface.AddMappingContext` _returnvalue_3 "/Game/shiza/input/shiza.shiza" 0 (struct)))))

(event `EnhancedInput|/Game/shiza/input/shizamoveinput`
  (params (ActionValue :type "Vector2D Structure") (ElapsedSeconds :type "Float (double-precision)") (TriggeredSeconds :type "Float (double-precision)") (InputAction :type "InputAction Object Reference" :default "/Game/shiza/input/shizamoveinput.shizamoveinput"))
  (bind (_returnvalue_roll _returnvalue_pitch _returnvalue_yaw) (`KismetMathLibrary.BreakRotator` (`self.GetControlRotation`)))
  (bind (_returnvalue_roll_2 _returnvalue_pitch_2 _returnvalue_yaw_2) (`KismetMathLibrary.BreakRotator` (`self.GetControlRotation`)))
  (:`Triggered`
    (`PlayerCameraManager.StartCameraShake` :`self` (`GameplayStatics.GetPlayerCameraManager` 0) :`ShakeClass` "/Script/GameplayCameras.DefaultCameraShakeBase" :`Scale` 3.0 :`PlaySpace` "World")
    (`self.AddMovementInput` (`KismetMathLibrary.GetRightVector` (`KismetMathLibrary.MakeRotator` _returnvalue_roll 0.0 _returnvalue_yaw)) ActionValue_Y)
    (`self.AddMovementInput` (`KismetMathLibrary.GetForwardVector` (`KismetMathLibrary.MakeRotator` _returnvalue_roll_2 0.0 _returnvalue_yaw_2)) ActionValue_X)))

(event `EnhancedInput|/Game/shiza/input/shizaleftclick`
  (params (ActionValue :type Boolean) (ElapsedSeconds :type "Float (double-precision)") (TriggeredSeconds :type "Float (double-precision)") (InputAction :type "InputAction Object Reference" :default "/Game/shiza/input/shizaleftclick.shizaleftclick"))
  (:`Started`
    (if (not (`PlayerController.bShowMouseCursor` (`GameplayStatics.GetPlayerController` 0)))
      (bind _returnvalue (`GameplayStatics.GetActorOfClass` "/Game/shiza/blueprints/bp_Fonariks.bp_Fonariks_C"))
      (`/Game/shiza/blueprints/bp_Fonariks.click` _returnvalue))))

(event `EnhancedInput|/Game/shiza/input/shizalookinput`
  (params (ActionValue :type "Vector2D Structure") (ElapsedSeconds :type "Float (double-precision)") (TriggeredSeconds :type "Float (double-precision)") (InputAction :type "InputAction Object Reference" :default "/Game/shiza/input/shizalookinput.shizalookinput"))
  (:`Triggered`
    (if (not (`PlayerController.bShowMouseCursor` (`GameplayStatics.GetPlayerController` 0)))
      (`self.AddControllerRollInput` ActionValue_X)
      (`self.AddControllerYawInput` (* ActionValue_Y -1.0)))))

(event `EnhancedInput|/Game/shiza/input/shizajumpinput`
  (params (ActionValue :type Boolean) (ElapsedSeconds :type "Float (double-precision)") (TriggeredSeconds :type "Float (double-precision)") (InputAction :type "InputAction Object Reference" :default "/Game/shiza/input/shizajumpinput.shizajumpinput"))
  (:`Triggered`
    (`self.Jump`)))

(event `self.ReceiveTick`
  (params (DeltaSeconds :type "Float (single-precision)"))
  (bind _returnvalue (`SceneComponent.K2_GetComponentLocation` (`self.Camera`)))
  (bind _outhit (`KismetSystemLibrary.LineTraceSingle` _returnvalue (+ (* (`SceneComponent.GetForwardVector` (`self.Camera`)) (500.0 500.0 500.0)) _returnvalue) "TraceTypeQuery1"))
  (cast `/Game/shiza/blueprints/bp_gl` (`.HitActor` (`GameplayStatics.BreakHitResult` _outhit))
    (:`then`
      (set `self.hover` true))
    (:`CastFailed`
      (set `self.hover` false)
      (set `self.glstable` self))))

(event `EnhancedInput|/Game/shiza/input/shizaE`
  (params (ActionValue :type Boolean) (ElapsedSeconds :type "Float (double-precision)") (TriggeredSeconds :type "Float (double-precision)") (InputAction :type "InputAction Object Reference" :default "/Game/shiza/input/shizaE.shizaE"))
  (bind _returnvalue (`SceneComponent.K2_GetComponentLocation` (`self.Camera`)))
  (:`Started`
    (bind _outhit (`KismetSystemLibrary.LineTraceSingle` _returnvalue (+ (* (`SceneComponent.GetForwardVector` (`self.Camera`)) (500.0 500.0 500.0)) _returnvalue) "TraceTypeQuery1"))
    (bind _asbp_gl (cast `/Game/shiza/blueprints/bp_gl` (`.HitActor` (`GameplayStatics.BreakHitResult` _outhit))))
    (cast `/Game/shiza/blueprints/bp_gl_stable` (`.HitActor` (`GameplayStatics.BreakHitResult` _outhit))
      (:`then`
        (`/Game/shiza/blueprints/bp_gl.on clicked` _asbp_gl self)
        (set `self.glstable` (`.HitActor` (`GameplayStatics.BreakHitResult` _outhit))))
      (:`CastFailed`
        (set `self.gl` (`.HitActor` (`GameplayStatics.BreakHitResult` _outhit)))
        (if (not (`self.is taking something`))
          (`/Game/shiza/blueprints/bp_gl.on clicked` _asbp_gl self)
          (set `self.is taking something` true))))))

(event `EnhancedInput|/Game/shiza/input/shizaGgrop`
  (params (ActionValue :type Boolean) (ElapsedSeconds :type "Float (double-precision)") (TriggeredSeconds :type "Float (double-precision)") (InputAction :type "InputAction Object Reference" :default "/Game/shiza/input/shizaGgrop.shizaGgrop"))
  (:`Started`
    (if (`self.is taking something`)
      (bind _asbp_gl (cast `/Game/shiza/blueprints/bp_gl` (`self.gl`)))
      (`/Game/shiza/blueprints/bp_gl.on grop` _asbp_gl)
      (set `self.is taking something` false))))

(fn `UserConstructionScript`)