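; Pickup flashlight actor that the player can carry, drop and switch on and off.
; OnClicked sets IsTake and makes the cube overlap WorldStatic; Tick then teleports it to the BP_CHARACTER pawn's location and rotation with a yaw offset, without attaching it.
; OnGrop drops it by lowering it, clearing IsTake and restoring blocking collision.
; Click toggles the RectLight intensity only while the item is held.
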(event `self.on clicked`
  (params (user :type "Actor Object Reference"))
  (`PrimitiveComponent.SetCollisionResponseToChannel` (`self.Cube`) "ECC_WorldStatic" "ECR_Overlap")
  (set `self.is take` true))

(event `self.on grop`
  (`self.K2_AddActorWorldOffset` (0.0 0.0 -50.0))
  (set `self.is take` false)
  (`PrimitiveComponent.SetCollisionResponseToChannel` (`self.Cube`) "ECC_WorldStatic" "ECR_Block"))

(event `self.ReceiveTick`
  (params (DeltaSeconds :type "Float (single-precision)"))
  (if (`self.is take`)
    (bind _asbp_character (cast `/Game/shiza/blueprints/BP_CHARACTER` (`GameplayStatics.GetPlayerPawn` 0)))
    (bind (_returnvalue_roll _returnvalue_pitch _returnvalue_yaw) (`KismetMathLibrary.BreakRotator` (`self.K2_GetActorRotation` _asbp_character)))
    (`self.K2_TeleportTo` (`self.K2_GetActorLocation` _asbp_character) (`KismetMathLibrary.MakeRotator` _returnvalue_roll _returnvalue_pitch (+ _returnvalue_yaw -70.0)))))

(fn `click`
  (if (`self.is take`)
    (if (`self.switcher`)
      (set `self.switcher` false)
      (`LightComponent.SetIntensity` (`self.RectLight`) 0.0)
      (else
        (set `self.switcher` true)
        (`LightComponent.SetIntensity` (`self.RectLight`) 9000.0)))))

(fn `UserConstructionScript`
  (`parent.UserConstructionScript`))